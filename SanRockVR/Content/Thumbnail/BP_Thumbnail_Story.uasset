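; Base Blueprint for a clickable VR story thumbnail, with an empty StartStoryPart event as the hook for launching a story part.
; On BeginPlay it caches the first StoryCanvas actor in the level.
; A click fires that hook, disables the thumbnail, then flags the button press and a tutorial step via SanVRPlayerController.
; Enable and Disable switch decal visibility and sphere collision together.
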(event Custom|StartStoryPart)

(event Custom|Enable
  (Rendering|SetVisibility (Variables|Default|GetDecal) true false)
  (Collision|SetCollisionEnabled (Variables|Default|GetSphere) "QueryAndPhysics"))

(event Custom|Disable
  (Rendering|SetVisibility (Variables|Default|GetDecal) false false)
  (Collision|SetCollisionEnabled (Variables|Default|GetSphere) "NoCollision"))

(event EventBeginPlay
  (|CallParentFunction)
  (bind _outactors (Actor|GetAllActorsOfClass "/Game/Animations/StoryCanvas.StoryCanvas_C"))
  (Variables|Default|SetStoryCanvas (Utilities|Array|Get(acopy) _outactors)))

(event Collision|EventActorBeginOverlap
  (params (OtherActor :type Actor%20Object%20Reference)))

(event EventTick
  (params (DeltaSeconds :type Float%20%28single-precision%29)))

(event EventButtonClicked
  (CallFunction|StartStoryPart)
  (Rendering|ToggleVisibility (Variables|Default|GetDecal) false)
  (CallFunction|Disable)
  (bind _asvrplayer_controller (Utilities|Casting|CastToSanVRPlayerController (Game|GetPlayerController 0)))
  (Variables|/Game/VirtualRealityBP/Blueprints/SanVRPlayerController.SanVRPlayerController_C|SetHasPressedVRButton _asvrplayer_controller true)
  (Utilities|Array|SetArrayElem (Variables|/Game/Animations/StoryCanvas.StoryCanvas_C|GetTutBools (Variables|/Game/VirtualRealityBP/Blueprints/SanVRPlayerController.SanVRPlayerController_C|GetStoryCanvasRef _asvrplayer_controller)) 2 true))

(fn ConstructionScript
  (|CallParentFunction))