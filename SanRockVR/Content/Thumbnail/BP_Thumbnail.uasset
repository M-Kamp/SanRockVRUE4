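; BP_Thumbnail is a base clickable thumbnail that shows its button states through a decal.
; BeginPlay gives the decal a dynamic material instance, whose "Highlight" vector parameter the events switch between highlight, base and pressed colors.
; Pressed saves the current color, and Released restores it before calling ButtonClicked, which only prints a placeholder message.
; StopHighlight also sets Selected to true, despite restoring the base color.
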(event Custom|Highlight
  (bind _asmaterial_instance_dynamic (Utilities|Casting|CastToMaterialInstanceDynamic (Variables|/Script/Engine.DecalComponent|GetDecalMaterial (Variables|Default|GetDecal))))
  (Rendering|Material|SetVectorParameterValue _asmaterial_instance_dynamic "Highlight" (Variables|Default|GetHighlightColor) :!class /Script/Engine.MaterialInstanceDynamic))

(event Custom|StopHighlight
  (bind _asmaterial_instance_dynamic (Utilities|Casting|CastToMaterialInstanceDynamic (Variables|/Script/Engine.DecalComponent|GetDecalMaterial (Variables|Default|GetDecal))))
  (Rendering|Material|SetVectorParameterValue _asmaterial_instance_dynamic "Highlight" (Variables|Default|GetBaseColor) :!class /Script/Engine.MaterialInstanceDynamic)
  (Variables|Default|SetSelected true))

(event Custom|Pressed
  (bind _asmaterial_instance_dynamic (Utilities|Casting|CastToMaterialInstanceDynamic (Variables|/Script/Engine.DecalComponent|GetDecalMaterial (Variables|Default|GetDecal))))
  (bind _returnvalue (Rendering|Material|GetVectorParameterValue _asmaterial_instance_dynamic "Highlight" :!class /Script/Engine.MaterialInstanceDynamic))
  (Variables|Default|SetLastColor _returnvalue)
  (Rendering|Material|SetVectorParameterValue _asmaterial_instance_dynamic "Highlight" (Variables|Default|GetPressedColor) :!class /Script/Engine.MaterialInstanceDynamic))

(event Custom|Released
  (bind _asmaterial_instance_dynamic (Utilities|Casting|CastToMaterialInstanceDynamic (Variables|/Script/Engine.DecalComponent|GetDecalMaterial (Variables|Default|GetDecal))))
  (Rendering|Material|SetVectorParameterValue _asmaterial_instance_dynamic "Highlight" (Variables|Default|GetLastColor) :!class /Script/Engine.MaterialInstanceDynamic)
  (CallFunction|ButtonClicked))

(event Custom|ButtonClicked
  (Development|PrintString "BaseClicked"))

(event EventBeginPlay
  (bind _returnvalue (Rendering|Material|CreateDynamicMaterialInstance (Variables|Default|GetDecal) :!class /Script/Engine.DecalComponent))
  (bind _output_get (Variables|Default|SetDecalMaterialInstance _returnvalue))
  (Rendering|Components|Decal|SetDecalMaterial (Variables|Default|GetDecal) _output_get))

(fn ConstructionScript)