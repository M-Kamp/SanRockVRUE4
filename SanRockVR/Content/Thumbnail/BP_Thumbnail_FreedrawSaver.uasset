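; BP_Thumbnail_FreedrawSaver is an in-world button actor that saves freedraw render targets on three walls.
; SetRefToWalls stores left, centre and right wall references.
; ButtonClicked calls SaveRenderTargetFreedraw on each in turn, nesting the checks so an invalid wall also skips those after it.
; Enable and Disable toggle the button's decal visibility and sphere collision.
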(event Custom|SetRefToWalls
  (params (Left :type Paintable%20Rock%20Rock%20Canvas%20Object%20Reference) (Centre :type Paintable%20Rock%20Rock%20Canvas%20Object%20Reference) (Right :type Paintable%20Rock%20Rock%20Canvas%20Object%20Reference))
  (Variables|Default|SetPR_Left Left)
  (Variables|Default|SetPR_Centre Centre)
  (Variables|Default|SetPR_Right Right))

(event Custom|Enable
  (Rendering|SetVisibility (Variables|Default|GetDecal) true false)
  (Collision|SetCollisionEnabled (Variables|Default|GetSphere) "QueryAndPhysics"))

(event Custom|Disable
  (Rendering|SetVisibility (Variables|Default|GetDecal) false false)
  (Collision|SetCollisionEnabled (Variables|Default|GetSphere) "NoCollision"))

(event EventBeginPlay
  (|CallParentFunction) ; This node is disabled and will not be called.\nDrag off pins to build functionality.
)

(event Collision|EventActorBeginOverlap
  (params (OtherActor :type Actor%20Object%20Reference)))

(event EventTick
  (params (DeltaSeconds :type Float%20%28single-precision%29)))

(event EventButtonClicked
  (bind _pr_right (Variables|Default|GetPR_Right))
  (bind _pr_left (Variables|Default|GetPR_Left))
  (bind _pr_centre (Variables|Default|GetPR_Centre))
  (Utilities|IsValid _pr_left
    (:Is%20Valid
      (Default|SaveRenderTargetFreedraw _pr_left)
      (Utilities|IsValid _pr_centre
        (:Is%20Valid
          (Default|SaveRenderTargetFreedraw _pr_centre)
          (Utilities|IsValid _pr_right
            (:Is%20Valid
              (Default|SaveRenderTargetFreedraw _pr_right))))))))

(fn ConstructionScript
  (|CallParentFunction))