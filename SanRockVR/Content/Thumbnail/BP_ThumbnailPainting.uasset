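; Thumbnail painting actor whose decal gets a dynamic material and changes its Highlight color for highlight, press and release.
; Press stores the current color for release to restore; Highlight clears Selected and StopHighlight sets it.
; Image persistence looks like test scaffolding: BeginPlay imports any Test.exr only to print its width, then saves a freshly cleared render target as "Test" in the screenshot directory.
; SaveImages is empty.
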(event Custom|Highlight
  (bind _asmaterial_instance_dynamic (Utilities|Casting|CastToMaterialInstanceDynamic (Variables|/Script/Engine.DecalComponent|GetDecalMaterial (Variables|Default|GetDecal))))
  (Rendering|Material|SetVectorParameterValue _asmaterial_instance_dynamic "Highlight" (Variables|Default|GetHighlightColor) :!class /Script/Engine.MaterialInstanceDynamic)
  (Variables|Default|SetSelected false))

(event Custom|StopHighlight
  (bind _asmaterial_instance_dynamic (Utilities|Casting|CastToMaterialInstanceDynamic (Variables|/Script/Engine.DecalComponent|GetDecalMaterial (Variables|Default|GetDecal))))
  (Rendering|Material|SetVectorParameterValue _asmaterial_instance_dynamic "Highlight" (Variables|Default|GetBaseColor) :!class /Script/Engine.MaterialInstanceDynamic)
  (Variables|Default|SetSelected true))

(event Custom|Pressed
  (bind _asmaterial_instance_dynamic (Utilities|Casting|CastToMaterialInstanceDynamic (Variables|/Script/Engine.DecalComponent|GetDecalMaterial (Variables|Default|GetDecal))))
  (bind _returnvalue (Rendering|Material|GetVectorParameterValue _asmaterial_instance_dynamic "Highlight" :!class /Script/Engine.MaterialInstanceDynamic))
  (Variables|Default|SetLastColor _returnvalue)
  (Rendering|Material|SetVectorParameterValue _asmaterial_instance_dynamic "Highlight" (Variables|Default|GetPressedColor) :!class /Script/Engine.MaterialInstanceDynamic))

(event Custom|Released
  (bind _asmaterial_instance_dynamic (Utilities|Casting|CastToMaterialInstanceDynamic (Variables|/Script/Engine.DecalComponent|GetDecalMaterial (Variables|Default|GetDecal))))
  (Rendering|Material|SetVectorParameterValue _asmaterial_instance_dynamic "Highlight" (Variables|Default|GetLastColor) :!class /Script/Engine.MaterialInstanceDynamic))

(event Custom|SaveImages)

(event Custom|LoadImages
  (bind _returnvalue (Class|BlueprintPathsLibrary|ScreenShotDir))
  (bind _returnvalue_2 (Utilities|String|Append _returnvalue "Test.exr"))
  (if (Class|BlueprintPathsLibrary|FileExists _returnvalue_2)
    (Development|PrintString "Exists")
    (bind _returnvalue_3 (Class|KismetRenderingLibrary|ImportFileasTexture2D _returnvalue_2))
    (Development|PrintString (Utilities|String|ToString(Integer) (Class|Texture2D|BlueprintGetSizeX _returnvalue_3)))
    (else
      (Development|PrintString "Does not exist"))))

(event EventBeginPlay
  (bind _returnvalue (Rendering|Material|CreateDynamicMaterialInstance (Variables|Default|GetDecal) :!class /Script/Engine.DecalComponent))
  (bind _output_get (Variables|Default|SetDecalMaterialInstance _returnvalue))
  (Rendering|Components|Decal|SetDecalMaterial (Variables|Default|GetDecal) _output_get)
  (CallFunction|LoadImages)
  (bind _returnvalue_2 (Rendering|CreateRenderTarget2D 256 256 "RTF_RGBA8" "(R=1.000000,G=0.025431,B=0.000000,A=1.000000)"))
  (Rendering|ClearRenderTarget2D _returnvalue_2 "(R=1.000000,G=0.000000,B=0.046303,A=1.000000)")
  (Class|ImageSaveLoad|SaveRenderTargettoDisk (Variables|Default|GetImageSaveLoad) _returnvalue_2 (Class|BlueprintPathsLibrary|ScreenShotDir) "Test"))

(fn ConstructionScript)