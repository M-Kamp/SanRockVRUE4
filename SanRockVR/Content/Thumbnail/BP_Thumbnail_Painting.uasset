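; Painting thumbnail button that holds render targets for the left, center and right paintable rock walls.
; Clicking it pushes those targets onto the wall references and has the SanVR player controller save all thumbnails.
; Helper functions create blank targets, draw saved pixel data into them through a material, or convert them back to pixel data.
; An older file-based export and import path, labeled old, remains alongside unconnected nodes.
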(event Custom|LoadImagesToRenderTargets
  ;[1 1 1] Old stuff
  (bind _asvrplayer_controller (Utilities|Casting|CastToSanVRPlayerController (Game|GetPlayerController 0)))
  (for (_array_element _array_index) (Utilities|Array|MakeArray (Variables|/Game/VirtualRealityBP/Blueprints/SanVRPlayerController.SanVRPlayerController_C|GetPaintableRockLeft _asvrplayer_controller) (Variables|/Game/VirtualRealityBP/Blueprints/SanVRPlayerController.SanVRPlayerController_C|GetPaintableRockCenter _asvrplayer_controller) (Variables|/Game/VirtualRealityBP/Blueprints/SanVRPlayerController.SanVRPlayerController_C|GetPaintableRockRight _asvrplayer_controller))
    (bind _returnvalue (Class|KismetRenderingLibrary|ImportFileasTexture2D (Utilities|String|Append (Class|KismetSystemLibrary|GetProjectSavedDirectory) (Utilities|String|Append (Utilities|String|ToString(Integer) (Variables|Default|GetThumbNailID)) (Utilities|String|ToString(Integer) (+ _array_index 1)) (Utilities|String|MakeLiteralString "IMG") (Variables|Default|GetExtension)))))
    (bind _returnvalue_2 (Rendering|CreateRenderTarget2D 256 256 "RTF_RGBA16f"))
    (bind _returnvalue_3 (Rendering|Material|CreateDynamicMaterialInstance "/Game/Thumbnail/M_TexToRenderTar.M_TexToRenderTar" "None" :!class /Script/Engine.KismetMaterialLibrary))
    (Rendering|Material|SetTextureParameterValue _returnvalue_3 "Texture" _returnvalue)
    (Rendering|DrawMaterialtoRenderTarget _returnvalue_2 _returnvalue_3)
    (bind _output_get (Variables|/Game/DrawingAssets/PaintableRock.PaintableRock_C|SetRendertexture _array_element _returnvalue_2))
    (Rendering|Material|SetTextureParameterValue (Variables|/Game/DrawingAssets/PaintableRock.PaintableRock_C|GetMatInstance _array_element) "RenderTarget" _output_get))
  (Development|PrintString "Loaded RTs from disk"))

(event Custom|InitNewRTandSave
  ;[1 1 1] Old stuff
  (bind _asvrplayer_controller (Utilities|Casting|CastToSanVRPlayerController (Game|GetPlayerController 0)))
  (for _array_element (Utilities|Array|MakeArray (Variables|/Game/VirtualRealityBP/Blueprints/SanVRPlayerController.SanVRPlayerController_C|GetPaintableRockLeft _asvrplayer_controller) (Variables|/Game/VirtualRealityBP/Blueprints/SanVRPlayerController.SanVRPlayerController_C|GetPaintableRockCenter _asvrplayer_controller) (Variables|/Game/VirtualRealityBP/Blueprints/SanVRPlayerController.SanVRPlayerController_C|GetPaintableRockRight _asvrplayer_controller))
    (bind _returnvalue (Rendering|CreateRenderTarget2D 256 256 "RTF_RGBA16f"))
    (bind _output_get (Variables|/Game/DrawingAssets/PaintableRock.PaintableRock_C|SetRendertexture _array_element _returnvalue))
    (Rendering|Material|SetTextureParameterValue (Variables|/Game/DrawingAssets/PaintableRock.PaintableRock_C|GetMatInstance _array_element) "RenderTarget" _output_get))
  (CallFunction|SaveImages (Variables|Default|GetThumbNailID)))

(event Custom|SetRefTOWalls
  (params (left :type Paintable%20Rock%20Rock%20Canvas%20Object%20Reference) (center :type Paintable%20Rock%20Rock%20Canvas%20Object%20Reference) (right :type Paintable%20Rock%20Rock%20Canvas%20Object%20Reference))
  (Variables|Default|SetPR_Left left)
  (Variables|Default|SetPR_Center center)
  (Variables|Default|SetPR_Right right))

(event Custom|SaveImages
  (params (ImageID :type Integer))
  (bind _returnvalue (Class|KismetSystemLibrary|GetProjectSavedDirectory))
  ;[1 1 1] Old stuff
  (bind _asvrplayer_controller (Utilities|Casting|CastToSanVRPlayerController (Game|GetPlayerController 0)))
  (for (_array_element _array_index) (Utilities|Array|MakeArray (Variables|/Game/VirtualRealityBP/Blueprints/SanVRPlayerController.SanVRPlayerController_C|GetPaintableRockLeft _asvrplayer_controller) (Variables|/Game/VirtualRealityBP/Blueprints/SanVRPlayerController.SanVRPlayerController_C|GetPaintableRockCenter _asvrplayer_controller) (Variables|/Game/VirtualRealityBP/Blueprints/SanVRPlayerController.SanVRPlayerController_C|GetPaintableRockRight _asvrplayer_controller))
    (Rendering|ExportRenderTarget (Variables|/Game/DrawingAssets/PaintableRock.PaintableRock_C|GetRendertexture _array_element) _returnvalue (Utilities|String|Append (Utilities|String|ToString(Integer) ImageID) (Utilities|String|ToString(Integer) (+ _array_index 1)) (Utilities|String|MakeLiteralString "IMG") (Variables|Default|GetExtension)))
    (Development|PrintString _returnvalue))
  (Development|PrintString "Saved RTs to disk"))

(event Custom|HandleImageLoading
  (bind _returnvalue (Class|KismetSystemLibrary|GetProjectSavedDirectory))
  (bind _returnvalue_2 (Utilities|String|MakeLiteralString "IMG"))
  (bind _returnvalue_3 (Utilities|String|MakeLiteralString "1"))
  (bind _extension (Variables|Default|GetExtension))
  (bind _thumbnailid (Variables|Default|GetThumbNailID))
  (bind _returnvalue_4 (Utilities|String|ToString(Integer) _thumbnailid))
  (bind _returnvalue_5 (Utilities|String|Append _returnvalue _returnvalue_4 _returnvalue_3 _returnvalue_2 _extension))
  ;[1 1 1] Old stuff
  (Development|PrintString _returnvalue_5)
  (if (Class|BlueprintPathsLibrary|FileExists _returnvalue_5)
    (Development|PrintString "Exists")
    (CallFunction|LoadImagestoRenderTargets)
    (else
      (Development|PrintString "Does not exist")
      (CallFunction|InitNewRTandSave))))

(event EventBeginPlay
  (|CallParentFunction))

(event EventButtonClicked
  (Default|SetRenderTargetUpdateRock (Variables|Default|GetPR_Left) (Variables|Default|GetLeftRT))
  (Default|SetRenderTargetUpdateRock (Variables|Default|GetPR_Center) (Variables|Default|GetCenterRT))
  (Default|SetRenderTargetUpdateRock (Variables|Default|GetPR_Right) (Variables|Default|GetRightRT))
  (bind _asvrplayer_controller (Utilities|Casting|CastToSanVRPlayerController (Game|GetPlayerController 0)))
  (Default|SaveAllThumbnails _asvrplayer_controller))

(fn ConstructionScript
  (|CallParentFunction))

(fn SetRenderTargets
  (params (Left :type Array%20of%20Color%20Structures) (Center :type Array%20of%20Color%20Structures) (Right :type Array%20of%20Color%20Structures))
  (Utilities|FlowControl|Sequence
    (:then_0
      (bind _returnvalue (Class|ImageSaveLoad|TexturefromImage (Variables|Default|GetImageSaveLoad) 256 256 Left true))
      (bind _returnvalue_2 (Rendering|Material|CreateDynamicMaterialInstance "/Game/Thumbnail/M_TexToRenderTar.M_TexToRenderTar" "None" :!class /Script/Engine.KismetMaterialLibrary))
      (bind _returnvalue_3 (Rendering|CreateRenderTarget2D 256 256 "RTF_RGBA16f"))
      (Variables|Default|SetLeftRT _returnvalue_3)
      (Rendering|Material|SetTextureParameterValue _returnvalue_2 "Texture" _returnvalue)
      (Rendering|DrawMaterialtoRenderTarget (Variables|Default|GetLeftRT) _returnvalue_2))
    (:then_1
      (bind _returnvalue_4 (Class|ImageSaveLoad|TexturefromImage (Variables|Default|GetImageSaveLoad) 256 256 Center true))
      (bind _returnvalue_5 (Rendering|Material|CreateDynamicMaterialInstance "/Game/Thumbnail/M_TexToRenderTar.M_TexToRenderTar" "None" :!class /Script/Engine.KismetMaterialLibrary))
      (bind _returnvalue_6 (Rendering|CreateRenderTarget2D 256 256 "RTF_RGBA16f"))
      (Variables|Default|SetCenterRT _returnvalue_6)
      (Rendering|Material|SetTextureParameterValue _returnvalue_5 "Texture" _returnvalue_4)
      (Rendering|DrawMaterialtoRenderTarget (Variables|Default|GetCenterRT) _returnvalue_5))
    (:then_2
      (bind _returnvalue_7 (Class|ImageSaveLoad|TexturefromImage (Variables|Default|GetImageSaveLoad) 256 256 Right true))
      (bind _returnvalue_8 (Rendering|Material|CreateDynamicMaterialInstance "/Game/Thumbnail/M_TexToRenderTar.M_TexToRenderTar" "None" :!class /Script/Engine.KismetMaterialLibrary))
      (bind _returnvalue_9 (Rendering|CreateRenderTarget2D 256 256 "RTF_RGBA16f"))
      (Variables|Default|SetRightRT _returnvalue_9)
      (Rendering|Material|SetTextureParameterValue _returnvalue_8 "Texture" _returnvalue_7)
      (Rendering|DrawMaterialtoRenderTarget (Variables|Default|GetRightRT) _returnvalue_8)
      (return))))

(fn InitNewRenderTargets
  (Utilities|FlowControl|Sequence
    (:then_0
      (bind _returnvalue (Rendering|CreateRenderTarget2D 256 256 "RTF_RGBA16f"))
      (bind _output_get (Variables|Default|SetLeftRT _returnvalue))
      (bind _returnvalue_2 (Class|ImageSaveLoad|TexturefromRT (Variables|Default|GetImageSaveLoad) _output_get)))
    (:then_1
      (bind _returnvalue_3 (Rendering|CreateRenderTarget2D 256 256 "RTF_RGBA16f"))
      (bind _output_get_2 (Variables|Default|SetCenterRT _returnvalue_3))
      (bind _returnvalue_4 (Class|ImageSaveLoad|TexturefromRT (Variables|Default|GetImageSaveLoad) _output_get_2)))
    (:then_2
      (bind _returnvalue_5 (Rendering|CreateRenderTarget2D 256 256 "RTF_RGBA16f"))
      (bind _output_get_3 (Variables|Default|SetRightRT _returnvalue_5))
      (bind _returnvalue_6 (Class|ImageSaveLoad|TexturefromRT (Variables|Default|GetImageSaveLoad) _output_get_3))
      (return _returnvalue_2 _returnvalue_4 _returnvalue_6))))

(fn ConvertRenderTargetsFColor
  (Utilities|FlowControl|Sequence
    (:then_0
      (bind _returnvalue (Class|ImageSaveLoad|TexturefromRT (Variables|Default|GetImageSaveLoad) (Variables|Default|GetLeftRT))))
    (:then_1
      (bind _returnvalue_2 (Class|ImageSaveLoad|TexturefromRT (Variables|Default|GetImageSaveLoad) (Variables|Default|GetCenterRT))))
    (:then_2
      (bind _returnvalue_3 (Class|ImageSaveLoad|TexturefromRT (Variables|Default|GetImageSaveLoad) (Variables|Default|GetRightRT)))
      (return _returnvalue _returnvalue_2 _returnvalue_3))))