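; BP_Thumbnail_Story_Start is a thumbnail Blueprint that starts the first part of the story when its StartStoryPart event is called.
; The event plays Scene 1 Part 1 on the StoryCanvas.
; It then casts player controller 0 to VRPlayerController, sets one tutorial flag in that controller's StoryCanvasRef and marks the tutorial completed.
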(event EventBeginPlay
  (|CallParentFunction) ; This node is disabled and will not be called.\nDrag off pins to build functionality.
)

(event EventStartStoryPart
  (Default|PlayScene1Part1 (Variables|Default|GetStoryCanvas))
  (bind _asvrplayer_controller (Utilities|Casting|CastToVRPlayerController (Game|GetPlayerController 0)))
  (Utilities|Array|SetArrayElem (Variables|/Game/Animations/StoryCanvas.StoryCanvas_C|GetTutBools (Variables|/Game/VirtualRealityBP/Blueprints/VRPlayerController.VRPlayerController_C|GetStoryCanvasRef _asvrplayer_controller)) 2 true)
  (Variables|/Game/VirtualRealityBP/Blueprints/VRPlayerController.VRPlayerController_C|SetHasCompletedTutorial _asvrplayer_controller true))

(fn ConstructionScript
  (|CallParentFunction))